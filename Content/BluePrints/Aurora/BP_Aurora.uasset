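; BP_Aurora is a spline-driven actor, presumably an aurora visual, built entirely in the Construction Script with no runtime logic.
; It adds an X-forward spline mesh for each spline segment, creating the first and last separately from the looped middle ones.
; The GetStartAndEndLocationAndTangent helper is meant to supply each segment's endpoints and tangents from adjacent spline points in local space.
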(fn `UserConstructionScript`
  (bind (_startlocation _starttangent _endlocation _endtangent) (`self.GetStartAndEndLocationAndTangent` 0))
  (bind (_startlocation_2 _starttangent_2 _endlocation_2 _endtangent_2) (`self.GetStartAndEndLocationAndTangent` (- (`SplineComponent.GetNumberOfSplinePoints` (`self.Spline`)) 2)))
  (bind _returnvalue (`AddComponent|NODE_AddSplineMeshComponent-3`))
  (`SplineMeshComponent.SetForwardAxis` _returnvalue "X" true)
  (`SplineMeshComponent.SetStartAndEnd` _returnvalue _startlocation _starttangent _endlocation _endtangent true)
  (for _index (range 1 (+ (- (`SplineComponent.GetNumberOfSplinePoints` (`self.Spline`)) 3) 1))
    (bind _returnvalue_2 (`AddComponent|NODE_AddSplineMeshComponent-0`))
    (`SplineMeshComponent.SetForwardAxis` _returnvalue_2 "X" true)
    (bind (_startlocation_3 _starttangent_3 _endlocation_3 _endtangent_3) (`self.GetStartAndEndLocationAndTangent` _index))
    (`SplineMeshComponent.SetStartAndEnd` _returnvalue_2 _startlocation_3 _starttangent_3 _endlocation_3 _endtangent_3 true))
  (bind _returnvalue_3 (`AddComponent|NODE_AddSplineMeshComponent-4`))
  (`SplineMeshComponent.SetForwardAxis` _returnvalue_3 "X" true)
  (`SplineMeshComponent.SetStartAndEnd` _returnvalue_3 _startlocation_2 _starttangent_2 _endlocation_2 _endtangent_2 true))