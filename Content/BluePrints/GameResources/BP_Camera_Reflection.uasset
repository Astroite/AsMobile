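; Camera reflection actor that renders a planar mirror view through the SCReflection scene capture into a render target.
; The construction script mirrors CMNormal's location across the horizontal ReflectionPlaneHeight and builds the capture's rotation from its axes reflected about world up.
; The capture transform is set only at construction; Tick just prints a CMNormal rotation component for debugging.
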(event `self.ReceiveActorBeginOverlap`
  (params (OtherActor :type "Actor Object Reference")))

(event `self.ReceiveTick`
  (params (DeltaSeconds :type "Float (single-precision)"))
  (`KismetSystemLibrary.PrintString` (`KismetStringLibrary.Conv_VectorToString` (`.Z` (`KismetMathLibrary.BreakRotIntoAxes` (`SceneComponent.K2_GetComponentRotation` (`self.CM_Normal`))))) true true (struct :`G` 0.66 :`B` 1.0 :`A` 1.0) 1000.0))

(fn `UserConstructionScript`
  (bind _returnvalue (`KismetMathLibrary.Vector_Up`))
  (bind _sc_reflection (`self.SC_Reflection`))
  (bind _cm_normal (`self.CM_Normal`))
  (set `SceneCaptureComponent2D.TextureTarget` (`self.RenderTarget`) _sc_reflection)
  (`SceneComponent.K2_SetWorldLocation` _sc_reflection (`KismetMathLibrary.MakeVector` (.x (`SceneComponent.K2_GetComponentLocation` _cm_normal)) (.y (`SceneComponent.K2_GetComponentLocation` _cm_normal)) (- (* (`self.ReflectionPlaneHeight`) 2.0) (.z (`SceneComponent.K2_GetComponentLocation` _cm_normal)))) false false)
  (`SceneComponent.K2_SetWorldRotation` _sc_reflection (`KismetMathLibrary.MakeRotationFromAxes` (`KismetMathLibrary.MirrorVectorByNormal` (`SceneComponent.GetForwardVector` _cm_normal) _returnvalue) (`KismetMathLibrary.MirrorVectorByNormal` (`SceneComponent.GetRightVector` _cm_normal) _returnvalue) (`KismetMathLibrary.MirrorVectorByNormal` (`SceneComponent.GetUpVector` _cm_normal) _returnvalue)) false false))