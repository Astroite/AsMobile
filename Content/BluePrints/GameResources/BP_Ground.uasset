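; BP_Ground is a ground actor that drives a scan effect from impact points through the MPC_FiberGround material parameter collection.
; On Hit, it writes the hit location to Origin, resets ScanTimer and sets IsHit.
; Each Tick advances ScanTimer by ScanSpeed times delta time, then clears IsHit once the next step would exceed one.
; All state lives in the collection, so a new hit restarts the single shared scan.
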(event `self.ReceiveTick`
  (params (DeltaSeconds :type "Float (single-precision)"))
  (bind _returnvalue (`KismetMaterialLibrary.GetScalarParameterValue` "/Game/Resources/Materials/MaterialParameters/MPC_FiberGround.MPC_FiberGround" "ScanSpeed"))
  (bind _returnvalue_2 (`KismetMaterialLibrary.GetScalarParameterValue` "/Game/Resources/Materials/MaterialParameters/MPC_FiberGround.MPC_FiberGround" "ScanTimer"))
  (bind _returnvalue_3 (+ _returnvalue_2 (* _returnvalue DeltaSeconds)))
  (if (<= _returnvalue_3 1.0)
    (`KismetMaterialLibrary.SetScalarParameterValue` "/Game/Resources/Materials/MaterialParameters/MPC_FiberGround.MPC_FiberGround" "ScanTimer" _returnvalue_3)
    (else
      (`KismetMaterialLibrary.SetScalarParameterValue` "/Game/Resources/Materials/MaterialParameters/MPC_FiberGround.MPC_FiberGround" "IsHit"))))

(event `self.ReceiveHit`
  (params (MyComp :type "PrimitiveComponent Object Reference") (Other :type "Actor Object Reference") (OtherComp :type "PrimitiveComponent Object Reference") (bSelfMoved :type Boolean) (HitLocation :type "Vector Structure") (HitNormal :type "Vector Structure") (NormalImpulse :type "Vector Structure") (Hit :type "HitResult Structure (by ref)"))
  (`KismetMaterialLibrary.SetVectorParameterValue` "/Game/Resources/Materials/MaterialParameters/MPC_FiberGround.MPC_FiberGround" "Origin" (`KismetMathLibrary.Conv_VectorToLinearColor` HitLocation))
  (`KismetMaterialLibrary.SetScalarParameterValue` "/Game/Resources/Materials/MaterialParameters/MPC_FiberGround.MPC_FiberGround" "ScanTimer")
  (`KismetMaterialLibrary.SetScalarParameterValue` "/Game/Resources/Materials/MaterialParameters/MPC_FiberGround.MPC_FiberGround" "IsHit" 1.0))

(fn `UserConstructionScript`)