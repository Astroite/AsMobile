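; Actor that maintains a player-following deformation render target for desert dunes, using an orthographic DeformCapture component.
; Each tick it moves to the player's XY snapped to capture texel size (256 across) and publishes location and delta time to MPC_Deform.
; It then draws a dynamic post-process material into the persistent target, passing the move as a normalized offset so accumulated deformation can scroll with the capture.
; Both render targets are cleared on begin and end play.
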(event `self.ReceiveBeginPlay`
  (`KismetMaterialLibrary.SetScalarParameterValue` "/Game/Assets/Material/Parameter/MPC_Deform.MPC_Deform" "DeformCaptureSize" (`SceneCaptureComponent2D.OrthoWidth` (`self.DeformCapture`)))
  (bind _returnvalue (`KismetMaterialLibrary.CreateDynamicMaterialInstance` "/Game/Assets/Material/Material/PostProcess/M_PP_DrawtoPresident.M_PP_DrawtoPresident"))
  (set `self.DrawMaterial` _returnvalue)
  (`KismetRenderingLibrary.ClearRenderTarget2D` "/Game/Assets/Solution/Desert/Tex/RT_DeformCapture.RT_DeformCapture")
  (`KismetRenderingLibrary.ClearRenderTarget2D` "/Game/Assets/Solution/Desert/Tex/RT_DeformPresident.RT_DeformPresident"))

(event `self.ReceiveEndPlay`
  (params (EndPlayReason :type "EEndPlayReason Enum" :default "Destroyed"))
  (`KismetRenderingLibrary.ClearRenderTarget2D` "/Game/Assets/Solution/Desert/Tex/RT_DeformCapture.RT_DeformCapture")
  (`KismetRenderingLibrary.ClearRenderTarget2D` "/Game/Assets/Solution/Desert/Tex/RT_DeformPresident.RT_DeformPresident"))

(event `self.ReceiveTick`
  (params (DeltaSeconds :type "Float (single-precision)"))
  (`self.Move Capture`)
  (`self.DrawToPersistent`)
  (`KismetMaterialLibrary.SetScalarParameterValue` "/Game/Assets/Material/Parameter/MPC_Deform.MPC_Deform" "DeltaTime" DeltaSeconds))

(fn `DrawToPersistent`
  (bind (_returnvalue_x _returnvalue_y) (`KismetMathLibrary.BreakVector2D` (/ (`self.MoveOffset`) (`SceneCaptureComponent2D.OrthoWidth` (`self.DeformCapture`)))))
  (`MaterialInstanceDynamic.SetVectorParameterValue` (`self.DrawMaterial`) "Offset" (make `LinearColor` _returnvalue_x _returnvalue_y 0.0 1.0))
  (`KismetRenderingLibrary.DrawMaterialToRenderTarget` "/Game/Assets/Solution/Desert/Tex/RT_DeformPresident.RT_DeformPresident" (`self.DrawMaterial`)))

(fn `Move Capture`
  (bind (_returnvalue_x _returnvalue_y) (`KismetMathLibrary.BreakVector` (`self.K2_GetActorLocation` (`GameplayStatics.GetPlayerCharacter` 0))))
  (bind (_returnvalue_x_2 _returnvalue_y_2) (`KismetMathLibrary.BreakVector` (- (`self.SnapToPixelWorldSize` _returnvalue_x _returnvalue_y (* (`SceneCaptureComponent2D.OrthoWidth` (`self.DeformCapture`)) (/ 1.0 256.0))) (`self.K2_GetActorLocation`))))
  (bind _output_get (set `self.MoveOffset` (`KismetMathLibrary.MakeVector2D` _returnvalue_x_2 _returnvalue_y_2)))
  (`self.K2_AddActorWorldOffset` (`KismetMathLibrary.MakeVector` (`KismetMathLibrary.BreakVector2D` _output_get) (`.Y` (`KismetMathLibrary.BreakVector2D` _output_get))))
  (`KismetMaterialLibrary.SetVectorParameterValue` "/Game/Assets/Material/Parameter/MPC_Deform.MPC_Deform" "CaptureLocation" (`KismetMathLibrary.Conv_VectorToLinearColor` (`self.K2_GetActorLocation`))))

(fn `UserConstructionScript`)